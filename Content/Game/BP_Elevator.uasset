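; Interactive multi-floor elevator actor whose construction script spawns linked BP_Floor child actors at 500-unit height intervals.
; Its elevator button disables player input and opens the UI_Etage floor widget, while the door button opens the doors.
; MoveFloor closes the doors, lerps the cabin to the target height with a timeline, then reopens them.
; Door opening also starts a five-second timer; random starting-floor logic is left disconnected.
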(event Custom|MoveFloor
  (params (targetFloor :type Integer))
  (bind _beginlocation_elevator (Variables|Default|GetBeginlocation%20Elevator))
  (bind (_x _y _z) (Math|Vector|BreakVector _beginlocation_elevator))
  (if (!= targetFloor (Variables|Default|GetCurentFloor))
    (CallFunction|CloseDoor)
    (Variables|Default|SetCurentFloor targetFloor)
    (Components|Timeline|SetPlayRate (Variables|Default|GetMoveelevator) 0.25)
    (Variables|Default|SetCurrent%20Location (Variables|/Script/Engine.SceneComponent|GetRelativeLocation (Variables|Default|Getelevator)))
    (bind _newtrack_0 (Timeline|Moveelevator PlayFromStart)
      (:Update
        (Transformation|SetRelativeLocation (Variables|Default|Getelevator) (Math|Vector|Lerp(Vector) (Variables|Default|GetCurrent%20Location) (Math|Vector|MakeVector _x _y (+ _z (* (Variables|Default|GetCurentFloor) 5e+02))) _newtrack_0) false false)
        (Development|PrintString (Utilities|String|ToString(Vector) (Math|Vector|MakeVector _x _y (+ _z (* (Variables|Default|GetCurentFloor) 5e+02))))))
      (:Finished
        (CallFunction|Opendoor)))
    (else
      (CallFunction|Opendoor))))

(event Custom|Opendoor
  (Variables|Default|SetcurrentLocationD1 (Variables|/Script/Engine.SceneComponent|GetRelativeLocation (Variables|Default|GetDoor1)))
  (Variables|Default|SetCurentLocationD2 (Variables|/Script/Engine.SceneComponent|GetRelativeLocation (Variables|Default|GetDoor2)))
  (Utilities|FlowControl|Sequence
    (:then_0
      (bind _door (Timeline|movedoor Play)
        (:Update
          (Transformation|SetRelativeLocation (Variables|Default|GetDoor1) (Math|Vector|Lerp(Vector) (Variables|Default|GetcurrentLocationD1) (Math|Vector|MakeVector 47.0 -5e+01 0.0) _door) false false)
          (Transformation|SetRelativeLocation (Variables|Default|GetDoor2) (Math|Vector|Lerp(Vector) (Variables|Default|GetCurentLocationD2) (Math|Vector|MakeVector 47.0 5e+01 0.0) _door) false false))
        (:Finished
          (Utilities|FlowControl|DoOnce false :!label _label
            (:Completed
              (Utilities|Time|SetTimerbyEvent (EventDispatchers|CreateEvent :!event Custom|CloseDoor) 5.0))))))
    (:then_1
      (goto _label Reset))))

(event Custom|CloseDoor
  (bind _door (Timeline|movedoor ReverseFromEnd)
    (:Update
      (Transformation|SetRelativeLocation (Variables|Default|GetDoor1) (Math|Vector|Lerp(Vector) (Variables|Default|GetcurrentLocationD1) (Math|Vector|MakeVector 47.0 -5e+01 0.0) _door) false false)
      (Transformation|SetRelativeLocation (Variables|Default|GetDoor2) (Math|Vector|Lerp(Vector) (Variables|Default|GetCurentLocationD2) (Math|Vector|MakeVector 47.0 5e+01 0.0) _door) false false))
    (:Finished
      (Utilities|FlowControl|DoOnce false
        (:Completed
          (Utilities|Time|SetTimerbyEvent (EventDispatchers|CreateEvent :!event Custom|CloseDoor) 5.0))))))

(event EventBeginPlay
  (Variables|Default|SetBeginlocation%20Elevator (Variables|/Script/Engine.SceneComponent|GetRelativeLocation (Variables|Default|Getelevator))))

(event EventInteraction
  (params (playerRef :type BP%20First%20Person%20Character%20Object%20Reference) (CompenentHit :type Actor%20Component%20Object%20Reference))
  (if (== CompenentHit (Variables|Default|GetBouttonElevator))
    (bind _output_get (Variables|Default|SetPlayer%20Ref playerRef))
    (bind _output_get_2 (Variables|Default|SetPlayerControllerRef (Game|GetPlayerController 0)))
    (Input|DisableInput _output_get _output_get_2)
    (Variables|/Script/Engine.PlayerController|SetbShowMouseCursor _output_get_2 true)
    (bind _returnvalue (UserInterface|CreateWidget "/Game/Game/UI_Etage.UI_Etage_C"))
    (bind _output_get_3 (Variables|Default|SetRefUI _returnvalue))
    (Variables|/Game/Game/UI_Etage.UI_Etage_C|SetRefElevator _output_get_3 self)
    (UserInterface|Viewport|AddtoViewport _output_get_3 0)
    (bind _output_get_4 (Variables|/Game/Game/UI_Etage.UI_Etage_C|SetFloor _output_get_3 (Variables|Default|GetCurentFloor)))
    (Default|SetEtage _output_get_3 _output_get_4)
    (elif (== CompenentHit (Variables|Default|GetBouttonDoor))
      (CallFunction|Opendoor))))

(fn ConstructionScript
  (bind _arrow (Variables|Default|GetArrow))
  (bind _returnvalue (Transformation|GetRelativeTransform _arrow))
  (bind (_x _y _z) (Math|Vector|BreakVector (.location _returnvalue)))
  (for _index (range 0 (Variables|Default|GetNombreEtage))
    (bind _returnvalue_2 (AddComponent|AddChildActorComponent false (Math|Transform|MakeTransform (Math|Vector|MakeVector _x _y (+ _z (* _index 500))) (.rotation _returnvalue) (.scale _returnvalue))))
    (ChildActorComponent|SetChildActorClass _returnvalue_2 "/Game/Game/BP_Floor.BP_Floor_C")
    (bind _asbp_floor (Utilities|Casting|CastToBP_Floor (Variables|/Script/Engine.ChildActorComponent|GetChildActor _returnvalue_2)))
    (Variables|/Game/Game/BP_Floor.BP_Floor_C|SetElevatorRef _asbp_floor self)
    (Variables|/Game/Game/BP_Floor.BP_Floor_C|Setfloor _asbp_floor _index)))